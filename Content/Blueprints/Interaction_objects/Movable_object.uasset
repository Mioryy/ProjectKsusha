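; Movable object actor that can be attached to a character so it moves with them.
; StartMovable attaches the root component to the passed reference's capsule, keeping its world location and rotation, and sets the mesh to ignore the Pawn collision channel.
; StopMavable detaches the actor in place and restores blocking against Pawns.
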(event `/Game/Blueprints/Interfaces/interface_movable.Stop_mavable`
  (`self.K2_DetachFromActor` "KeepWorld" "KeepWorld" "KeepWorld")
  (`PrimitiveComponent.SetCollisionResponseToChannel` (`self.StaticMesh`) "ECC_Pawn" "ECR_Block"))

(fn `Start_movable`
  (params (Reference :type "Character Object Reference"))
  (returns (Resualt :type Boolean))
  (bind _returnvalue (`SceneComponent.K2_AttachToComponent` (`self.DefaultSceneRoot`) (`Character.CapsuleComponent` Reference) "None" "KeepWorld" "KeepWorld" "KeepRelative" true))
  (`PrimitiveComponent.SetCollisionResponseToChannel` (`self.StaticMesh`) "ECC_Pawn" "ECR_Ignore")
  (return _returnvalue))

(fn `UserConstructionScript`)