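; Air trap actor that pushes an overlapping BP_Character_Human upward inside a box volume.
; Begin overlap stores the character, and Tick applies an upward movement force that fades with height from the actor's origin toward the box top.
; End overlap zeroes the character's vertical velocity and clears the reference.
; The construction script raises the box by its half-height so it sits on the actor's origin.
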(event `self.ReceiveTick`
  (params (DeltaSeconds :type "Float (single-precision)"))
  (bind (_returnvalue_x _returnvalue_y _returnvalue_z) (`KismetMathLibrary.BreakVector` (`self.K2_GetActorLocation`)))
  (bind _newvar_0 (`self.NewVar_0`))
  (bind (_returnvalue_x_2 _returnvalue_y_2 _returnvalue_z_2) (`KismetMathLibrary.BreakVector` (`self.K2_GetActorLocation` _newvar_0)))
  (if (`self.Overlap`)
    (`CharacterMovementComponent.AddForce` (`Character.CharacterMovement` _newvar_0) (`KismetMathLibrary.MakeVector` 0.0 0.0 (* (`KismetMathLibrary.Abs` (- (/ (`KismetMathLibrary.Abs` (- _returnvalue_z_2 _returnvalue_z)) (* (.z (`BoxComponent.BoxExtent` (`self.Box`))) 2.0)) 1.0)) 20000.0)))))

(event `self.Box.OnComponentBeginOverlap`
  (params (OverlappedComponent :type "PrimitiveComponent Object Reference") (OtherActor :type "Actor Object Reference") (OtherComp :type "PrimitiveComponent Object Reference") (OtherBodyIndex :type Integer) (bFromSweep :type Boolean) (SweepResult :type "HitResult Structure (by ref)"))
  (bind _asbp_character_human (cast `/Game/SideScrollerBP/Blueprints/BP_Character_Human` OtherActor))
  (set `self.Overlap` true)
  (set `self.NewVar_0` _asbp_character_human))

(event `self.Box.OnComponentEndOverlap`
  (params (OverlappedComponent :type "PrimitiveComponent Object Reference") (OtherActor :type "Actor Object Reference") (OtherComp :type "PrimitiveComponent Object Reference") (OtherBodyIndex :type Integer))
  (bind _newvar_0 (`self.NewVar_0`))
  (bind (_returnvalue_x _returnvalue_y) (`KismetMathLibrary.BreakVector` (`self.GetVelocity` _newvar_0)))
  (cast `/Game/SideScrollerBP/Blueprints/BP_Character_Human` OtherActor)
  (set `self.Overlap` false)
  (set `MovementComponent.Velocity` (`KismetMathLibrary.MakeVector` _returnvalue_x _returnvalue_y) (`Character.CharacterMovement` _newvar_0))
  (set `self.NewVar_0` null))

(fn `UserConstructionScript`
  (bind _box (`self.Box`))
  (`SceneComponent.K2_SetRelativeLocation` _box (`KismetMathLibrary.MakeVector` 0.0 0.0 (.z (`BoxComponent.BoxExtent` _box))) true true))