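; BP_Laders is an interactable ladder that puts a human character into its crawl state, apparently used for climbing.
; Interaction calls StartCrawl on the instigating BP_Character_Human.
; When that character leaves the Box1 volume, it calls StopCrawl and applies a movement force along the Arrow's forward vector.
; The construction script positions the Cube and Box1 from the LocationLaders and LocationBox variables.
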(event `self.Box1.OnComponentEndOverlap`
  (params (OverlappedComponent :type "PrimitiveComponent Object Reference") (OtherActor :type "Actor Object Reference") (OtherComp :type "PrimitiveComponent Object Reference") (OtherBodyIndex :type Integer))
  (bind _asbp_character_human (cast `/Game/SideScrollerBP/Blueprints/BP_Character_Human` OtherActor))
  (`/Game/SideScrollerBP/Blueprints/BP_Character_Human.StopCrawl` _asbp_character_human)
  (`CharacterMovementComponent.AddForce` (`Character.CharacterMovement` _asbp_character_human) (* (`SceneComponent.GetForwardVector` (`self.Arrow`)) 100000.0)))

(fn `interaction`
  (params (Instigator :type "Actor Object Reference"))
  (returns (result :type Boolean))
  (bind _asbp_character_human (cast `/Game/SideScrollerBP/Blueprints/BP_Character_Human` Instigator)
    (:`then`
      (`/Game/SideScrollerBP/Blueprints/BP_Character_Human.StartCrawl` _asbp_character_human))
    (:`CastFailed`
      (return false))))

(fn `UserConstructionScript`
  (`SceneComponent.K2_SetRelativeTransform` (`self.Cube`) (`self.Location_laders`) false false)
  (`SceneComponent.K2_SetRelativeLocation` (`self.Box1`) (`self.Location_box`) false false))